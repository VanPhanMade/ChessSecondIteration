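; BP_King is the king chess piece actor, and its graph adds sound feedback for piece interactions.
; On BeginPlay it binds handlers to its move, pickup and take dispatchers.
; Each handler plays a one-shot audio event in world space: a thud at the destination square, a pop or slash at the king's own location.
; No movement or rule logic lives in this graph.
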(event Custom|OnMovePiece_Event
  (params (DesiredMoveSquare :type Board%20Square%20Object%20Reference))
  (Class|FMODBlueprintStatics|PlayEventatLocation "/Game/FMOD/Events/ChessThud.ChessThud" (Math|Conversions|ToTransform(Vector) (Transformation|GetActorLocation DesiredMoveSquare))))

(event Custom|OnTakeThisPiece_Event
  (params (CurrentBoardSquare :type Board%20Square%20Object%20Reference))
  (Class|FMODBlueprintStatics|PlayEventatLocation "/Game/FMOD/Events/Slash.Slash" (Math|Conversions|ToTransform(Vector) (Transformation|GetActorLocation))))

(event Custom|OnPickupPiece_Event
  (Class|FMODBlueprintStatics|PlayEventatLocation "/Game/FMOD/Events/BubblePop.BubblePop" (Math|Conversions|ToTransform(Vector) (Transformation|GetActorLocation))))

(event EventBeginPlay
  (EventDispatchers|AssignOnMovePiece (delegate Custom|OnMovePiece_Event))
  (EventDispatchers|AssignOnPickupPiece (delegate Custom|OnPickupPiece_Event))
  (EventDispatchers|AssignOnTakeThisPiece (delegate Custom|OnTakeThisPiece_Event)))

(fn ConstructionScript)